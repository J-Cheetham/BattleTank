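; Player-controllable tank Blueprint that binds input to aiming, firing, movement and camera rotation.
; On BeginPlay it hands the barrel and turret to the aiming component and both tracks to the movement component.
; Drive and fire inputs are forwarded to those components.
; Aim axes rotate a separate azimuth gimbal for yaw and the spring arm for pitch, without directly turning the turret or barrel.
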(event `self.ReceiveBeginPlay`
  (`TankAimingComponent.Initialise` (`self.TankAiming1`) (`self.TankBarrel`) (`self.TankTurret`))
  (`TankMovementComponent.Initialise` (`self.TankMovement1`) (`self.TankTrack Left`) (`self.TankTrack Right`)))

(event `InputAxis|Aim Azimuth`
  (params (AxisValue :type "Float (single-precision)"))
  (`SceneComponent.K2_AddLocalRotation` (`self.Azimuth Gimbal`) (`KismetMathLibrary.MakeRotator` 0.0 0.0 AxisValue) false false))

(event `InputAxis|Aim Elevation`
  (params (AxisValue :type "Float (single-precision)"))
  (`SceneComponent.K2_AddLocalRotation` (`self.SpringArm1`) (`KismetMathLibrary.MakeRotator` 0.0 AxisValue) false false))

(event `InputAction|Fire`
  (params (Key :type "Key Structure"))
  (:`Pressed`
    (`TankAimingComponent.Fire` (`self.TankAiming1`))))

(event `InputAxis|MoveForward`
  (params (AxisValue :type "Float (single-precision)"))
  (`TankMovementComponent.IntendMoveForward` (`self.TankMovement1`) AxisValue))

(event `InputAxis|TurnRight`
  (params (AxisValue :type "Float (single-precision)"))
  (`TankMovementComponent.IntendTurnRight` (`self.TankMovement1`) AxisValue))

(fn `UserConstructionScript`)